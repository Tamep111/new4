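; BP_Blocks is a Blueprint that lays out static mesh components in a flat grid.
; Its construction script runs nested loops over X and Y, adding one mesh per cell at the loop indices multiplied by the Pedding spacing.
; The event graph holds only disabled placeholder events, so all of its logic sits in the construction script.
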(event EventBeginPlay)

(event Collision|EventActorBeginOverlap
  (params (OtherActor :type Actor%20Object%20Reference)))

(event EventTick
  (params (DeltaSeconds :type Float%20%28single-precision%29)))

(fn ConstructionScript
  (for _index (range 0 (Math|Float|Truncate (Math|Conversions|ToFloat(Integer) (Variables|Default|GetX))))
    (for _index_2 (range 0 (Math|Float|Truncate (Math|Conversions|ToFloat(Integer) (Variables|Default|GetY))))
      (AddComponent|AddStaticMeshComponent false (Math|Transform|MakeTransform (Math|Vector|MakeVector (* _index (Variables|Default|GetPedding)) (* _index_2 (Variables|Default|GetPedding)) 0.0))))))