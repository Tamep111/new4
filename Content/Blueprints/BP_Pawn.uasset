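; Player paddle pawn for what appears to be a Breakout-style game: it moves sideways with sweep and manages balls and lives.
; SpawnBall launches a crash sphere while lives remain, spending one and binding to its death event.
; Helper functions apply bonuses: extra ball, life changes, wall spawning and paddle widening.
; Widening repositions the cube near track edges, where it also starts a retriggerable timer restoring scale and material.
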(event Custom|SetDefScale
  (Utilities|FlowControl|RetriggerableDelay 6.0)
  (Transformation|SetActorScale3D (Variables|Default|GetBasicPawnScale))
  (Rendering|Material|SetMaterial (Variables|Default|GetCube) 0 "/Engine/MapTemplates/Materials/BasicAsset03.BasicAsset03"))

(event EventBeginPlay
  (Utilities|FlowControl|Sequence
    (:then_0
      (Input|SetInputModeGameOnly (Game|GetPlayerController 0) false))
    (:then_1
      (CallFunction|SpawnBall))))

(event Input|AxisEvents|InputAxisMoveSides
  (params (AxisValue :type Float%20%28single-precision%29))
  (Transformation|AddActorWorldOffset (Math|Vector|MakeVector (* AxisValue (Variables|Default|GetPawnSpeed) (Utilities|Time|GetWorldDeltaSeconds)) 0.0 0.0) true))

(event Input|KeyboardEvents|Escape
  (params (Key :type Key%20Structure :default "None"))
  (:Pressed
    (Game|QuitGame 0 "Quit" false)))

(fn ConstructionScript)

(fn PawnScale
  (bind _returnvalue (Transformation|GetActorLocation))
  (bind _returnvalue_2 (Transformation|GetActorLocation))
  (bind _basicpawnscale (Variables|Default|GetBasicPawnScale))
  (Transformation|SetActorScale3D (Math|Vector|MakeVector (+ (.x _basicpawnscale) 4.0) (.y _basicpawnscale) (.z _basicpawnscale)))
  (Rendering|Material|SetMaterial (Variables|Default|GetCube) 0 "/Engine/MapTemplates/Materials/BasicAsset01.BasicAsset01")
  (if (< (.x _returnvalue) 3e+03)
    (Transformation|SetWorldTransform (Variables|Default|GetCube) (Math|Transform|MakeTransform (Math|Vector|MakeVector 3.05e+03 (.y _returnvalue) (.z _returnvalue)) "0, 0, 0" (Transformation|GetActorScale3D)) false true)
    (CallFunction|SetDefScale :!label _label)
    (elif (> (.x _returnvalue_2) 6.2e+03)
      (Transformation|SetWorldTransform (Variables|Default|GetCube) (Math|Transform|MakeTransform (Math|Vector|MakeVector 6.15e+03 (.y _returnvalue_2) (.z _returnvalue_2)) "0, 0, 0" (Transformation|GetActorScale3D)) false true)
      (goto _label))))

(fn SpawnBall
  (if (not (< (Variables|Default|GetLife) 1))
    (bind _returnvalue (Game|SpawnActorfromClass "/Game/Blueprints/BP_Crash_Sphere.BP_Crash_Sphere_C" (Math|Conversions|ToTransform(Vector) (Transformation|GetWorldLocation (Variables|Default|GetCapsule))) "AdjustIfPossibleButAlwaysSpawn" "MultiplyWithRoot" 0 0))
    (bind _result (Math|Integer|DecrementInt (Variables|Default|GetLife))
      (:%20%20
        (bind _output_get (Variables|Default|SetLife _result))
        (Development|PrintString (Utilities|String|ToString(Integer) _output_get) true true "(R=1.000000,G=0.177017,B=0.186965,A=1.000000)")
        (bind _output_get_2 (Variables|Default|SetSphere _returnvalue))
        (EventDispatchers|BindEventtoOnDead _output_get_2 (EventDispatchers|CreateEvent :!event SpawnBall))
        (return)))))

(fn SpawnBonusBall
  (Game|SpawnActorfromClass "/Game/Blueprints/BP_Crash_Sphere_Child.BP_Crash_Sphere_Child_C" (Math|Conversions|ToTransform(Vector) (Transformation|GetWorldLocation (Variables|Default|GetCapsule))) "AdjustIfPossibleButAlwaysSpawn" "MultiplyWithRoot" 0 0)
  (return))

(fn BonusLife
  (bind _result (Math|Integer|IncrementInt (Variables|Default|GetLife))
    (:%20%20
      (Variables|Default|SetLife _result))))

(fn Minuslife
  (bind _result (Math|Integer|DecrementInt (Variables|Default|GetLife))
    (:%20%20
      (bind _output_get (Variables|Default|SetLife _result))
      (Development|PrintString (Utilities|String|ToString(Integer) _output_get) true true "(R=0.726656,G=1.000000,B=0.072390,A=1.000000)"))))

(fn SpawnWall
  (Game|SpawnActorfromClass "/Game/Blueprints/BP_Wall.BP_Wall_C" (Math|Transform|MakeTransform "4582.000000,4355.000000,151.000000" "0, 0, 0" "1.000000,1.000000,1.000000") "AlwaysSpawn" "MultiplyWithRoot" 0 0))